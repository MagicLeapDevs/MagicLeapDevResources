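; XR demo pawn that presents intro pages in Intro_P and steps through a looping sequence of XR tool demo levels.
; A camera-following, lerped widget shows front-end pages in the intro, or a level-name title elsewhere with the controller hidden.
; Tick line-traces a laser beam and dot, while the right trigger clicks through widget interaction.
; Level advance is blocked during intro pages and loads the next map when the confirm sound finishes.
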(event `self.ReceiveBeginPlay`
  (bind _motioncontroller (`self.MotionController`))
  ;[1 0 1] Begin Play. Get name of level, chop it up, and put it into the widget in order to denote which tool is being demoed.
  (`|ExecutionSequence`
    (:`then_0`
      (`SceneComponent.SetWorldScale3D` (`self.Widget`) (`KismetMathLibrary.Conv_DoubleToVector` (`self.WidgetScale`))))
    (:`then_1`
      (bind _returnvalue (`|CreateWidget` "/Game/UI/Widget_Header.Widget_Header_C"))
      (set `self.HeaderWidget` _returnvalue)
      (bind _returnvalue_2 (`|CreateWidget` "/Game/UI/W_Page_TitleScreen.W_Page_TitleScreen_C"))
      (set `self.TitleScreenWidget` _returnvalue_2)
      (bind _returnvalue_3 (`|CreateWidget` "/Game/UI/W_Page_Overview.W_Page_Overview_C"))
      (set `self.OverviewPage` _returnvalue_3)
      (bind _returnvalue_4 (`|CreateWidget` "/Game/UI/W_Page_Instructions.W_Page_Instructions_C"))
      (set `self.InstructionsPage` _returnvalue_4)
      (bind _returnvalue_5 (`|CreateWidget` "/Game/UI/W_Page_Controls.W_Page_Controls_C"))
      (set `self.ControlsPage` _returnvalue_5)
      (bind _returnvalue_6 (`|CreateWidget` "/Game/UI/W_Page_Legal.W_Page_Legal_C"))
      (set `self.LegalPage` _returnvalue_6))
    (:`then_2`
      (bind _returnvalue_7 (`GameplayStatics.GetCurrentLevelName` true))
      (switch `string` _returnvalue_7
        (:`Default`
          (set `self.EnableIntroScreens` false)
          (`WidgetComponent.SetWidget` (`self.Widget`) (`self.HeaderWidget`))
          (`self.SetWidget to Level Name`)
          (`SceneComponent.SetHiddenInGame` (`self.MotionController`) true true))
        (:`Intro_P`
          (set `self.EnableIntroScreens` true)
          (`WidgetComponent.SetWidget` (`self.Widget`) (`self.TitleScreenWidget`)))))
    (:`then_3`
      (`/Engine/EditorBlueprintResources/StandardMacros.IsValid` _motioncontroller
        (:`Is Valid`
          (set `MotionControllerComponent.MotionSource` "AnyHand" _motioncontroller))))))

(event `SetWidget to Level Name`
  ;[0 0 0] Sets the header Widget to the name of the Level/Tool
  (`WidgetComponent.SetWidget` (`self.Widget`) (`self.HeaderWidget`))
  (bind _aswidget_header (cast `/Game/UI/Widget_Header` (`WidgetComponent.GetUserWidgetObject` (`self.Widget`)))
    (:`then`
      (bind _returnvalue (`GameplayStatics.GetCurrentLevelName` true))
      (if (`KismetStringLibrary.NotEqual_StrStr` _returnvalue "Intro_P")
        (`KismetSystemLibrary.PrintString` _returnvalue false)
        (`TextBlock.SetText` (`/Game/UI/Widget_Header.TextBlock_Title` _aswidget_header) (`KismetTextLibrary.Conv_StringToText` (`KismetStringLibrary.LeftChop` _returnvalue 2)))
        (`TextBlock.SetText` (`/Game/UI/Widget_Header.TextBlock_BodyText` _aswidget_header) "")))
    (:`CastFailed`
      (`KismetSystemLibrary.PrintString` "FAIL" false))))

(event `self.ReceiveTick`
  (params (DeltaSeconds :type "Float (single-precision)"))
  ;[1 0 1] Tick
  (`self.WidgetSoftlock` DeltaSeconds)
  (`self.fLaserPointer`))

(event `InputAction|ResetApplication`
  (params (Key :type "Key Structure"))
  ;[0 0 0] Reset Application
  (:`Pressed`
    (`GameplayStatics.OpenLevel` "Intro_P")))

(event `WidgetSoftlock`
  (params (DeltaSeconds :type "Float (double-precision)"))
  (bind _returnvalue (`GameplayStatics.GetPlayerCameraManager` 0))
  (bind _widget (`self.Widget`))
  (bind _returnvalue_2 (`SceneComponent.K2_GetComponentLocation` _widget))
  (bind _returnvalue_3 (`PlayerCameraManager.GetCameraLocation` _returnvalue))
  ;[0 0 0] Widget Softlock. Interps between current position and positon from previous tick
  (bind _output_get (set `self.LocationTarget` (+ _returnvalue_3 (* (`self.GetActorForwardVector` _returnvalue) (`self.WidgetDistance`)))))
  (bind _output_get_2 (set `self.LocationCurrent` _returnvalue_2))
  (`SceneComponent.K2_SetWorldLocation` _widget (`KismetMathLibrary.VLerp` _output_get_2 _output_get (* DeltaSeconds (`self.WidgetInterpSpeed`))) false false)
  (`SceneComponent.K2_SetWorldRotation` _widget (`KismetMathLibrary.FindLookAtRotation` _returnvalue_2 _returnvalue_3) false false))

(event `Key|MotionController_Right_Trigger`
  (params (Key :type "Key Structure"))
  (bind _widgetinteraction (`self.WidgetInteraction`))
  ;[0 0 0] Pointer Widget Interaction Mapping
  (:`Pressed`
    (`WidgetInteractionComponent.PressPointerKey` _widgetinteraction "LeftMouseButton"))
  (:`Released`
    (`WidgetInteractionComponent.ReleasePointerKey` _widgetinteraction "LeftMouseButton")))

(event `AdvanceFrontEndScreens`
  (bind _widget (`self.Widget`))
  ;[0 0 1] Title Screen, Overview, Instructions, Controls
  (if (`self.EnableIntroScreens`)
    (bind _result (`/Engine/EditorBlueprintResources/StandardMacros.IncrementInt` (`self.PageIndex`))
      (:`  `
        (switch `int` _result
          (:`0`
            (`WidgetComponent.SetWidget` _widget (`self.TitleScreenWidget`))
            (`SceneComponent.SetVisibility` _widget true true)
            (`GameplayStatics.PlaySound2D` "/Game/UI/ui_confirm_short.ui_confirm_short" 1.0 1.0 0.0 null null :!label _label)
            (`KismetSystemLibrary.PrintString` (`KismetStringLibrary.Conv_IntToString` (`self.PageIndex`)) false))
          (:`1`
            (`WidgetComponent.SetWidget` _widget (`self.OverviewPage`))
            (goto _label))
          (:`2`
            (`WidgetComponent.SetWidget` _widget (`self.InstructionsPage`))
            (goto _label))
          (:`3`
            (`WidgetComponent.SetWidget` _widget (`self.ControlsPage`))
            (goto _label))
          (:`4`
            (`WidgetComponent.SetWidget` _widget (`self.LegalPage`))
            (goto _label))
          (:`5`
            (`SceneComponent.SetVisibility` _widget false true)
            (set `self.EnableIntroScreens` false)
            (set `self.PageIndex` -1)
            (`self.LoadNextLevel`)))))
    (else
      (`self.LoadNextLevel`))))

(event `LoadNextLevel`
  ;[0 0 0] Switching between tools, (levels.)
  (if (not (`self.EnableIntroScreens`)) :!label _label_2
    (`MagicLeapControllerFunctionLibrary.PlayHapticPattern` "Right" "ForceDown" "Low")
    (bind _returnvalue (`GameplayStatics.SpawnSound2D` "/Game/UI/ui_confirm_short.ui_confirm_short" 1.0 1.0 0.0 null))
    (add `AudioComponent.OnAudioFinished` _returnvalue (delegate `LoadNewTool`))))

(event `InputAction|LoadNextLevel`
  (params (Key :type "Key Structure"))
  ;[0 0 0] Switching between tools, (levels.)
  (:`Pressed`
    (goto _label_2)))

(event `LoadNewTool`
  ;[0 0 0] Switching between tools, (levels.)
  (bind _returnvalue (`GameplayStatics.GetCurrentLevelName` true))
  (switch `string` _returnvalue
    (:`Intro_P`
      (`GameplayStatics.OpenLevel` "AmbientBoost_P"))
    (:`AmbientBoost_P`
      (`GameplayStatics.OpenLevel` "CaptureOffset_P"))
    (:`CaptureOffset_P`
      (`GameplayStatics.OpenLevel` "ClipPlaneVisualizer_P"))
    (:`ClipPlaneVisualizer_P`
      (`GameplayStatics.OpenLevel` "HandTracking_P"))
    (:`HandTracking_P`
      (`GameplayStatics.OpenLevel` "LaserPointer_P"))
    (:`LaserPointer_P`
      (`GameplayStatics.OpenLevel` "Meshing_P"))
    (:`Meshing_P`
      (`GameplayStatics.OpenLevel` "Vignette_P"))
    (:`Vignette_P`
      (`GameplayStatics.OpenLevel` "Intro_P"))))

(fn `fLaserPointer`
  (bind _motioncontroller (`self.MotionController`))
  (bind _beammesh (`self.BeamMesh`))
  (bind _dotmesh (`self.DotMesh`))
  (bind _beamlength (`self.BeamLength`))
  (bind _returnvalue (`SceneComponent.K2_GetComponentLocation` _motioncontroller))
  (bind _returnvalue_2 (* (`self.BeamThickness`) 0.01))
  (bind _outhit (`KismetSystemLibrary.LineTraceSingle` :`Start` _returnvalue :`End` (+ (* (`SceneComponent.GetForwardVector` _motioncontroller) (`self.TraceDistance`)) _returnvalue) :`TraceChannel` "TraceTypeQuery1" :`TraceColor` (struct :`G` 0.5 :`B` 1.0 :`A` 1.0)))
  (if (`GameplayStatics.BreakHitResult` _outhit)
    (set `self.HitActor` (`.HitActor` (`GameplayStatics.BreakHitResult` _outhit)))
    (bind _output_get (set `self.BeamLengthNew` (* (* (/ (- (`.Distance` (`GameplayStatics.BreakHitResult` _outhit)) (`self.BeamOriginOffset`)) _beamlength) _beamlength) 0.01)))
    (`SceneComponent.SetWorldScale3D` _beammesh (`KismetMathLibrary.MakeVector` _returnvalue_2 _returnvalue_2 _output_get))
    (`SceneComponent.SetHiddenInGame` _dotmesh false false)
    (else
      (set `self.HitActor` null)
      (bind _output_get_2 (set `self.BeamLengthNew` (* (`self.BeamLength`) 0.01)))
      (`SceneComponent.SetWorldScale3D` _beammesh (`KismetMathLibrary.MakeVector` _returnvalue_2 _returnvalue_2 _output_get_2))
      (`SceneComponent.SetHiddenInGame` _dotmesh true false)))
  (`SceneComponent.K2_SetRelativeLocation` _beammesh (`KismetMathLibrary.MakeVector` (`KismetMathLibrary.Abs` (+ (* (`self.BeamLengthNew`) 0.5 100.0) (`self.BeamOriginOffset`)))) false false)
  (`MaterialInstanceDynamic.SetScalarParameterValue` (`self.BeamMaterial`) "GradientFalloffUVs" (/ (`self.BeamLengthNew`) (* (`self.BeamFadeLength`) 0.01)))
  (`SceneComponent.K2_SetWorldLocationAndRotation` (`self.DotMesh`) (`.Location` (`GameplayStatics.BreakHitResult` _outhit)) (`KismetMathLibrary.MakeRotator` (.roll (`KismetMathLibrary.Conv_VectorToRotator` (`.Normal` (`GameplayStatics.BreakHitResult` _outhit)))) (+ (.pitch (`KismetMathLibrary.Conv_VectorToRotator` (`.Normal` (`GameplayStatics.BreakHitResult` _outhit)))) 90.0) (.yaw (`KismetMathLibrary.Conv_VectorToRotator` (`.Normal` (`GameplayStatics.BreakHitResult` _outhit))))) false false))

(fn `fLaserPointerConstruction`
  (bind _beammesh (`self.BeamMesh`))
  (bind _beamlength (`self.BeamLength`))
  (bind _returnvalue (* (`self.BeamThickness`) 0.01))
  (bind _returnvalue_2 (* _beamlength 0.01))
  (`|ExecutionSequence`
    (:`then_0`
      (`SceneComponent.SetWorldScale3D` _beammesh (`KismetMathLibrary.MakeVector` _returnvalue _returnvalue _returnvalue_2))
      (`SceneComponent.K2_SetRelativeLocation` _beammesh (`KismetMathLibrary.MakeVector` (`KismetMathLibrary.Abs` (+ (* _beamlength 0.5) (* (`self.BeamOriginOffset`) 1.0)))) false false)
      (`SceneComponent.SetWorldScale3D` (`self.DotMesh`) (`KismetMathLibrary.Conv_DoubleToVector` (* (`self.DotSize`) 0.01))))
    (:`then_1`
      (bind _returnvalue_3 (`PrimitiveComponent.CreateDynamicMaterialInstance` (`self.BeamMesh`) 0 "/Game/ToolsR1/LaserPointerTool/M_Laser.M_Laser" "None"))
      (bind _output_get (set `self.BeamMaterial` _returnvalue_3))
      (`MaterialInstanceDynamic.SetScalarParameterValue` _output_get "GlobalTiling" _returnvalue_2)
      (`MaterialInstanceDynamic.SetScalarParameterValue` _output_get "GradientFalloffUVs" (/ _returnvalue_2 (* (`self.BeamFadeLength`) 0.01)))
      (`MaterialInstanceDynamic.SetVectorParameterValue` _output_get "Color" (`self.BeamColor`))
      (`MaterialInstanceDynamic.SetScalarParameterValue` _output_get "Emissive" (`self.BeamEmissive`)))
    (:`then_2`
      (bind _returnvalue_4 (`PrimitiveComponent.CreateDynamicMaterialInstance` (`self.DotMesh`) 0 "/Game/ToolsR1/LaserPointerTool/M_LaserDot.M_LaserDot" "None"))
      (bind _output_get_2 (set `self.DotMaterial` _returnvalue_4))
      (`MaterialInstanceDynamic.SetVectorParameterValue` _output_get_2 "Color" (`self.BeamColor`))
      (`MaterialInstanceDynamic.SetScalarParameterValue` _output_get_2 "Emissive" (`self.BeamEmissive`)))))

(fn `UserConstructionScript`
  ;[0 0 0] If this isn't the Intro Persistent level, scale the widget down to a singularity to hide it.
  (`|ExecutionSequence`
    (:`then_0`
      (bind _returnvalue (`GameplayStatics.GetCurrentLevelName` true))
      (if (`KismetStringLibrary.NotEqual_StrStr` _returnvalue "Intro_P")
        (`SceneComponent.SetWorldScale3D` (`self.Widget`) (0.0 0.0 0.0))))
    (:`then_1`
      (`self.fLaserPointerConstruction`))))