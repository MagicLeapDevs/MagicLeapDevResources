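; Tool actor that shifts the capture image through a post-process U/V offset, with optional trackpad tuning at runtime.
; Construction creates dynamic instances of the offset and frame materials, adds them as blendables, and applies the offset and debug-frame settings.
; When tuning is enabled, right motion-controller thumbstick axes increment the offsets, updating the material and widget readout.
; Tick keeps that widget ahead of the player camera, facing it.
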(event `self.ReceiveBeginPlay`
  (`SceneComponent.SetVisibility` (`self.Widget`) (`self.EnableTrackpadTuning`) false))

(event `self.ReceiveTick`
  (params (DeltaSeconds :type "Float (single-precision)"))
  (bind _returnvalue (`GameplayStatics.GetPlayerCameraManager` 0))
  (bind _widgetroot (`self.WidgetRoot`))
  (bind _returnvalue_2 (`self.K2_GetActorLocation` _returnvalue))
  ;[1 0 1] Tick. Update Widget Transform
  (`SceneComponent.K2_SetWorldLocation` _widgetroot (+ _returnvalue_2 (* (`self.GetActorForwardVector` _returnvalue) 50.0)) false false)
  (`SceneComponent.K2_SetWorldRotation` (`self.Widget`) (`KismetMathLibrary.FindLookAtRotation` (`SceneComponent.K2_GetComponentLocation` _widgetroot) _returnvalue_2) false false))

(event `InputAxisKey|MotionController_Right_Thumbstick_X`
  (params (AxisValue :type "Float (single-precision)"))
  (bind _asw_capture_offset (cast `/Game/ToolsR1/CaptureOffsetTool/W_CaptureOffset` (`WidgetComponent.GetUserWidgetObject` (`self.Widget`)) :!pure true))
  ;[0 0 0] Update offset values and adjust post process material parameters
  (if (`self.EnableTrackpadTuning`)
    (bind _output_get (set `self.Offset_U` (+ (* AxisValue -0.025) (`self.Offset_U`))))
    (`MaterialInstanceDynamic.SetScalarParameterValue` (`self.CaptureOffsetMaterial`) "Offset_U" _output_get)
    (`KismetSystemLibrary.PrintString` (`KismetStringLibrary.Concat_StrStr` "U: " (`KismetStringLibrary.Conv_DoubleToString` _output_get) "  |  " "V: " (`KismetStringLibrary.Conv_DoubleToString` (stale `InputAxisKey|MotionController_Right_Thumbstick_Y` _output_get))) false :!label _label)
    ;[0 0 0] Update Widget with current offset values
    (`TextBlock.SetText` (`/Game/ToolsR1/CaptureOffsetTool/W_CaptureOffset.TextBlock_UCoordinate` _asw_capture_offset) (`KismetTextLibrary.Conv_DoubleToText` (`self.Offset_U`) "HalfToEven"))
    (`TextBlock.SetText` (`/Game/ToolsR1/CaptureOffsetTool/W_CaptureOffset.TextBlock_VCoordinate` _asw_capture_offset) (`KismetTextLibrary.Conv_DoubleToText` (`self.Offset_V`) "HalfToEven"))))

(event `InputAxisKey|MotionController_Right_Thumbstick_Y`
  (params (AxisValue :type "Float (single-precision)"))
  ;[0 0 0] Update offset values and adjust post process material parameters
  (if (`self.EnableTrackpadTuning`)
    (bind _output_get (set `self.Offset_V` (+ (* AxisValue 0.025) (`self.Offset_V`))))
    (`MaterialInstanceDynamic.SetScalarParameterValue` (`self.CaptureOffsetMaterial`) "Offset_V" _output_get)
    (goto _label)))

(fn `UserConstructionScript`
  (bind _postprocess (`self.PostProcess`))
  (bind _captureoffsetmaterial (`self.CaptureOffsetMaterial`))
  (`|ExecutionSequence`
    (:`then_0`
      ;[0 0 0] Create Dynamic Material Instances of Offset and Frame Post Process Materials
      (set `PostProcessComponent.bEnabled` (`self.EnabledCaptureOffset`) _postprocess)
      (bind _returnvalue (`KismetMaterialLibrary.CreateDynamicMaterialInstance` "/Game/ToolsR1/CaptureOffsetTool/M_CaptureOffsetPP.M_CaptureOffsetPP"))
      (bind _output_get (set `self.CaptureOffsetMaterial` _returnvalue))
      (`PostProcessComponent.AddOrUpdateBlendable` _postprocess _output_get 1.0)
      (bind _returnvalue_2 (`KismetMaterialLibrary.CreateDynamicMaterialInstance` "/Game/ToolsR1/CaptureOffsetTool/M_CaptureFramePP.M_CaptureFramePP"))
      (bind _output_get_2 (set `self.CaptureFrameMaterial` _returnvalue_2))
      (`PostProcessComponent.AddOrUpdateBlendable` _postprocess _output_get_2 1.0))
    (:`then_1`
      ;[0 0 0] Draw Debug Frame controls.
      (`MaterialInstanceDynamic.SetScalarParameterValue` (`self.CaptureFrameMaterial`) "DebugFrame" (`KismetMathLibrary.Conv_BoolToDouble` (`self.DebugFrame`))))
    (:`then_2`
      ;[0 0 0] Set Offset Parameters in Details Panel
      (bind _output_get_3 (set `self.Offset_U` (`self.Offset_U`)))
      (`MaterialInstanceDynamic.SetScalarParameterValue` _captureoffsetmaterial "Offset_U" _output_get_3)
      (bind _output_get_4 (set `self.Offset_V` (`self.Offset_V`)))
      (`MaterialInstanceDynamic.SetScalarParameterValue` _captureoffsetmaterial "Offset_V" _output_get_4))))