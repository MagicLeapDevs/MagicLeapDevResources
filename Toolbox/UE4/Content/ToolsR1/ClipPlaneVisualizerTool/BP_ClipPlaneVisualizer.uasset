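; BP_ClipPlaneVisualizer is a tool Blueprint that visualizes clip plane and safe distances through a post-process effect.
; The construction script toggles the PostProcess component and adds a dynamic instance of M_ClipPlaneVisualizer as a full-weight blendable.
; It feeds the Blueprint's distance and banded-color settings into the material's scalar parameters, negating the clip plane distance.
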(fn `UserConstructionScript`
  (bind _postprocess (`self.PostProcess`))
  ;[0 0 0] Create Dynamic material Instances, set values
  (set `PostProcessComponent.bEnabled` (`self.IsEnabled`) _postprocess)
  (bind _returnvalue (`KismetMaterialLibrary.CreateDynamicMaterialInstance` "/Game/ToolsR1/ClipPlaneVisualizerTool/M_ClipPlaneVisualizer.M_ClipPlaneVisualizer"))
  (bind _output_get (set `self.ClipPlaneVisualizerMaterial` _returnvalue))
  (`PostProcessComponent.AddOrUpdateBlendable` _postprocess _output_get 1.0)
  (`MaterialInstanceDynamic.SetScalarParameterValue` _output_get "DistanceSafe" (`self.SafeDistance`))
  (`MaterialInstanceDynamic.SetScalarParameterValue` _output_get "DistanceClipPlane" (* (`self.ClipPlaneDistance`) -1.0))
  (`MaterialInstanceDynamic.SetScalarParameterValue` _output_get "UseBandedColors" (`KismetMathLibrary.Conv_BoolToDouble` (`self.UseBandedColors`)))
  (`MaterialInstanceDynamic.SetScalarParameterValue` _output_get "NumBandedColors" (`KismetMathLibrary.Conv_IntToDouble` (`self.NumBandedColors`))))